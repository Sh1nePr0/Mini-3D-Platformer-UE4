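; Main player character Blueprint that handles the lose condition.
; Every Tick, it sets Health to zero if the mesh falls to or below a world height threshold.
; That fall, or Health otherwise reaching zero, pauses the game, adds the Lose widget to the viewport, switches to UI-only input and shows the mouse cursor.
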(event EventBeginPlay)

(event Collision|EventActorBeginOverlap
  (params (OtherActor :type Actor%20Object%20Reference)))

(event EventTick
  (params (DeltaSeconds :type Float%20%28single-precision%29))
  (bind _returnvalue (Game|GetPlayerController 0))
  (if (<= (.Z (Math|Vector|BreakVector (Transformation|GetWorldLocation (Variables|Character|GetMesh)))) -6e+02)
    (Variables|Default|SetHealth 0.0)
    (Game|SetGamePaused true :!label _label)
    (bind _returnvalue_2 (UserInterface|CreateWidget "/Game/HUD/Lose.Lose_C" _returnvalue))
    (UserInterface|Viewport|AddtoViewport _returnvalue_2 0)
    (Input|SetInputModeUIOnly _returnvalue _returnvalue_2 "DoNotLock")
    (Variables|/Script/Engine.PlayerController|SetbShowMouseCursor _returnvalue true)
    (elif (<= (Variables|Default|GetHealth) 0.0)
      (goto _label))))

(fn ConstructionScript)